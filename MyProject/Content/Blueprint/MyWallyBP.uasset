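; MyWallyBP is an input-handling Blueprint that gives the player a noise-making action and opens the pause menu.
; Pressing F calls MakeNoise with the player pawn as instigator and plays a sound at that pawn's location.
; Pressing Escape creates the PauseScreen widget if no valid cached reference exists, adds it to the viewport, switches to UI-only input with a visible cursor, and pauses the game.
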(event `Key|F`
  (params (Key :type "Key Structure"))
  (bind _returnvalue (`GameplayStatics.GetPlayerPawn` 0))
  (:`Pressed`
    (`self.MakeNoise` 1.0 _returnvalue)
    (`GameplayStatics.PlaySoundAtLocation` null (`self.K2_GetActorLocation` _returnvalue) (struct) 1.0 1.0 0.0 null null null)))

(event `Key|Escape`
  (params (Key :type "Key Structure"))
  (bind _returnvalue (`GameplayStatics.GetPlayerController` 0))
  (bind _pausemenureference (`self.PauseMenuReference`))
  (:`Pressed`
    (`/Engine/EditorBlueprintResources/StandardMacros.IsValid` (`self.PauseMenuReference`)
      (:`Is Valid`
        _)
      (:`Is Not Valid`
        (bind _returnvalue_2 (`|CreateWidget` "/Game/Blueprint/PauseScreen.PauseScreen_C"))
        (set `self.PauseMenuReference` _returnvalue_2)))
    (`WidgetBlueprintLibrary.SetInputMode_UIOnlyEx` _returnvalue _pausemenureference)
    (set `PlayerController.bShowMouseCursor` true _returnvalue)
    (`UserWidget.AddToViewport` _pausemenureference 0)
    (`GameplayStatics.SetGamePaused` true)))

(fn `UserConstructionScript`)